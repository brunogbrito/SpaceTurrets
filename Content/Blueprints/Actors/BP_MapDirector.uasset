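; Map director actor that handles level transitions, world HUD display and level creator UI for a stage-based grid game.
; Timelines lerp the map borders to a new size, then rebuild the grid and spawn stage actors, or restart the game at default size.
; Grid, spawning and asset-loading functions are defined outside these graphs, which only trigger them, create widgets and forward score and stage updates.
; The construction script retains an unused slot-layout prototype.
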(event EventAddTextRender
  (params (RelativeLocation :type Vector :default "0, 0, 0") (CellIndex :type Integer))
  (bind _returnvalue (AddComponent|AddTextRenderComponent false (Math|Transform|MakeTransform RelativeLocation "90.000000,180.000000,0.000000" "1,1,1")))
  (Rendering|Components|TextRender|SetText _returnvalue (Utilities|Text|ToText(Integer) CellIndex)))

(event EventBeginPlay
  (|CallParentFunction))

(event EventInitializeLevelCreatorWidget
  (bind _returnvalue (UserInterface|CreateWidget "/Game/Widgets/WBP_LevelCreator.WBP_LevelCreator_C" (Game|GetPlayerController 0)))
  (UserInterface|Viewport|AddtoViewport _returnvalue 0))

(event EventInitializeLevelAssets
  (Class|STMapDirector|LoadLevelAssetsMap (Variables|Default|GetBP_TMap))
  (Variables|Default|SetGameStages (Variables|Default|GetBP_LevelStages)))

(event EventResetMapSize
  (if (== (Variables|Default|GetMapSize) 1e+03)
    (Variables|Default|SetMapSize 1e+03 :!label _label)
    (Class|STMapDirector|RestartGame)
    (else
      (bind _newtrack_0 (Timeline|Timeline_0 PlayFromStart)
        (:Update
          (Class|STMapDirector|InitializeMapBorders (Math|Float|Lerp (Variables|Default|GetMapSize) 1e+03 _newtrack_0)))
        (:Finished
          (goto _label))))))

(event EventInitializeWorldHUD
  (bind _returnvalue (UserInterface|CreateWidget "/Game/Widgets/WBP_WorldHUD.WBP_WorldHUD_C" (Game|GetPlayerController 0)))
  (bind _output_get (Variables|Default|SetW_HUD _returnvalue))
  (UserInterface|SetWidget (Variables|Default|GetHUD) _output_get))

(event EventUpdateHUDScore
  (params (NewScore :type Integer))
  (Default|UpdateScoreIndex (Variables|Default|GetW_HUD) NewScore))

(event EventSetNextLevel
  (params (NewMapSize :type Float%20%28single-precision%29) (Stage :type Integer))
  (bind _newtrack_0 (Timeline|PlayResizer PlayFromStart)
    (:Update
      (Class|STMapDirector|InitializeMapBorders (Math|Float|Lerp (Variables|Default|GetMapSize) NewMapSize _newtrack_0)))
    (:Finished
      (Variables|Default|SetMapSize NewMapSize)
      (Class|STMapDirector|InitializeGrid)
      (Class|STMapDirector|SpawnLevelActors Stage))))

(event EventUpdateHUDStage
  (params (NewStage :type Integer))
  (Default|UpdateStageIndex (Variables|Default|GetW_HUD) NewStage))

(event EventStartHUDAnimation
  (Default|StartAnimation (Variables|Default|GetW_HUD)))

(fn ConstructionScript
  (|CallParentFunction))